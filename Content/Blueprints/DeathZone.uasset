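; DeathZone is an actor that kills the player's run on overlap and reloads from the saved checkpoint.
; Any overlapping actor triggers it: player input is disabled, a DeathScreen widget appears, and the GameInstance's TimeSave counts down over three one-second delays.
; It then loads the "Test" save slot, copies saved location and score into MyGameInstance, opens the saved level and resets TimeSave.
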(event `self.ReceiveActorBeginOverlap`
  (params (OtherActor :type "Actor Object Reference"))
  (bind _returnvalue (`GameplayStatics.GetPlayerController` 0))
  (`self.DisableInput` (`GameplayStatics.GetPlayerPawn` 0) _returnvalue)
  (bind _returnvalue_2 (`|CreateWidget` "/Game/UI/DeathScreen.DeathScreen_C" _returnvalue))
  (`UserWidget.AddToViewport` _returnvalue_2 0)
  (bind _asmy_game_instance (cast `/Game/Blueprints/MyGameInstance` (`GameplayStatics.GetGameInstance`)))
  (`KismetSystemLibrary.Delay` 1.0)
  (set `/Game/Blueprints/MyGameInstance.TimeSave` (- (`/Game/Blueprints/MyGameInstance.TimeSave` _asmy_game_instance) 1) _asmy_game_instance)
  (`KismetSystemLibrary.Delay` 1.0)
  (set `/Game/Blueprints/MyGameInstance.TimeSave` (- (`/Game/Blueprints/MyGameInstance.TimeSave` _asmy_game_instance) 1) _asmy_game_instance)
  (`KismetSystemLibrary.Delay` 1.0)
  (set `/Game/Blueprints/MyGameInstance.TimeSave` (- (`/Game/Blueprints/MyGameInstance.TimeSave` _asmy_game_instance) 1) _asmy_game_instance)
  (bind _returnvalue_3 (`GameplayStatics.LoadGameFromSlot` "Test"))
  (bind _assave (cast `/Game/Blueprints/Save` _returnvalue_3))
  (bind _asmy_game_instance_2 (cast `/Game/Blueprints/MyGameInstance` (`GameplayStatics.GetGameInstance`)))
  (set `/Game/Blueprints/MyGameInstance.LocationSpawn` (`/Game/Blueprints/Save.Location_Save` _assave) _asmy_game_instance_2)
  (set `/Game/Blueprints/MyGameInstance.LoadingScore` (`/Game/Blueprints/Save.Score_Save` _assave) _asmy_game_instance_2)
  (`GameplayStatics.OpenLevel` (`KismetStringLibrary.Conv_StringToName` (`/Game/Blueprints/Save.Level_Save` _assave)))
  (`self.EnableInput` null)
  (set `/Game/Blueprints/MyGameInstance.TimeSave` 3 _asmy_game_instance))

(fn `UserConstructionScript`)